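; Health pickup that reacts when a first-person character overlaps its sphere, then destroys itself.
; The overlap checks for an exact BP_FirstPersonCharacter class match, then takes player character 0 rather than the overlapping actor.
; It passes that player's Health plus a fixed bonus to the health widget reference's UpdateHealthBar, without setting Health in this Blueprint.
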(event OnComponentBeginOverlap(Sphere)
  (params (OverlappedComponent :type Primitive%20Component%20Object%20Reference) (OtherActor :type Actor%20Object%20Reference) (OtherComp :type Primitive%20Component%20Object%20Reference) (OtherBodyIndex :type Integer) (bFromSweep :type Boolean) (SweepResult :type Hit%20Result%20Structure%20%28by%20ref%29))
  (if (== (Utilities|GetClass OtherActor) "/Game/FirstPerson/Blueprints/BP_FirstPersonCharacter.BP_FirstPersonCharacter_C")
    (bind _asbp_first_person_character (Utilities|Casting|CastToBP_FirstPersonCharacter (Game|GetPlayerCharacter 0)))
    (bind _output_get (Variables|Default|SetPlayerRef _asbp_first_person_character))
    (Default|UpdateHealthBar (Variables|/Game/FirstPerson/Blueprints/BP_FirstPersonCharacter.BP_FirstPersonCharacter_C|GetPlayerHealthREF _output_get) (+ (Variables|/Game/FirstPerson/Blueprints/BP_FirstPersonCharacter.BP_FirstPersonCharacter_C|GetHealth _output_get) 25.0))
    (Actor|DestroyActor)))

(fn ConstructionScript)